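; NPC AI controller that runs a guard behavior tree and tracks a perceived target for it.
; On BeginPlay it sets up the PatrolData blackboard, caches a reference to it and starts GuardBehavior.
; AI perception updates write sensed actors without the "Enemy" tag to the EnemyKey blackboard value, and clear that key when such an actor is no longer sensed.
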(event OnTargetPerceptionUpdated(AIPerception)
  (params (Actor :type Actor%20Object%20Reference) (Stimulus :type AI%20Stimulus%20Structure))
  (if (not (Actor|ActorHasTag Actor "Enemy"))
    (Variables|Default|SetStimulus Stimulus)
    (if (.bsuccessfullysensed (Variables|Default|GetStimulus))
      (AI|Components|Blackboard|SetValueasObject (Variables|Default|GetBlackboardReference) (Variables|Default|GetEnemyKey) Actor)
      (else
        (AI|Components|Blackboard|ClearValue (Variables|Default|GetBlackboardReference) (Variables|Default|GetEnemyKey))))))

(event EventBeginPlay
  (bind _blackboardcomponent (Class|AIController|UseBlackboard "/Game/Dynamic/NPC/AI/PatrolData.PatrolData"))
  (Variables|Default|SetBlackboardReference _blackboardcomponent)
  (AI|RunBehaviorTree "/Game/Dynamic/NPC/AI/GuardBehavior.GuardBehavior"))

(fn ConstructionScript)